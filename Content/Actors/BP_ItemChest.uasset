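; BP_ItemChest is an interactable chest that gives the interacting pawn a Key gameplay tag.
; Each Interact alternates between playing and reversing the AnimateLid timeline through a FlipFlop.
; Timeline updates pitch the lid mesh and add the tag to the pawn's ActionComponent active tags on every update, not once.
; When the timeline finishes, it activates the particle system.
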(event EventInteract
  (params (InstigatorPawn :type Pawn%20Object%20Reference))
  (Utilities|FlowControl|FlipFlop
    (:A
      (bind _pitch (Timeline|AnimateLid Play)
        (:Update
          (Transformation|SetRelativeRotation (Variables|Default|GetLidMesh) (Math|Rotator|MakeRotator 0.0 _pitch 0.0) false false)
          (GameplayTags|AddGameplayTag (Variables|/Script/Abstraction.ActionComponent|GetActiveGameplayTags (Actor|GetComponentbyClass InstigatorPawn "/Script/Abstraction.ActionComponent")) (Variables|Default|GetKey) :!class /Script/GameplayTags.BlueprintGameplayTagLibrary))
        (:Finished
          (Components|Activation|Activate (Variables|Default|GetParticleSystem) false))))
    (:B
      (Timeline|AnimateLid Reverse))))

(fn ConstructionScript)