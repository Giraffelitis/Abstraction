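; Base player character Blueprint that sets up input and relays objective updates to the HUD.
; On BeginPlay it adds keyboard/mouse and gamepad Enhanced Input mapping contexts, then creates the objectives list widget.
; Objective events forward list updates to that widget, and info and completion messages to WBPObjectivesUI, which is not assigned in these graphs.
; Camera pitch limits and spring-arm panning toward an attractor are present but disconnected.
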(event Custom|CreateObjectiveWidget
  ;[1 1 1] Objectives List HUD
  (bind _returnvalue (UserInterface|CreateWidget "/Game/Widgets/WBP_Objectives.WBP_Objectives_C" (Game|GetPlayerController 0)))
  (UserInterface|Viewport|AddtoViewport _returnvalue 0)
  (Variables|Default|SetWBP_Objectives _returnvalue))

(event EventBeginPlay
  (bind _asplayer_controller (Utilities|Casting|CastToPlayerController (Pawn|GetController)))
  (Input|AddMappingContext (PlayerController|LocalPlayerSubsystems|GetEnhancedInputLocalPlayerSubsystem _asplayer_controller) "/Game/Input/ICM_KBMDefaults.ICM_KBMDefaults" 0 "(bIgnoreAllPressedKeysUntilRelease=True,bForceImmediately=False)")
  (Input|AddMappingContext (PlayerController|LocalPlayerSubsystems|GetEnhancedInputLocalPlayerSubsystem _asplayer_controller) "/Game/Input/ICM_GamepadDefaults.ICM_GamepadDefaults" 0 "(bIgnoreAllPressedKeysUntilRelease=True,bForceImmediately=False)")
  (CallFunction|CreateObjectiveWidget))

(event EventOnShowObjectiveCompleted
  (params (Message :type Text%20%28by%20ref%29))
  (bind _wbp_objectivesui (Variables|Default|GetWBP_ObjectivesUI))
  ;[1 1 1] Show Objective Completed
  (if (Utilities|IsValid _wbp_objectivesui)
    (Default|ShowObjectiveCompleted _wbp_objectivesui Message)))

(event EventOnShowObjectiveInfo
  (params (Objective :type Objective%20Data%20Structure))
  (bind _wbp_objectivesui (Variables|Default|GetWBP_ObjectivesUI))
  ;[1 1 1] Show Objective Info
  (if (Utilities|IsValid _wbp_objectivesui)
    (Default|ShowObjectiveInfo _wbp_objectivesui (.Message (Utilities|Struct|BreakObjectiveData Objective)))))

(event EventOnShowUpdatedObjectiveList
  (params (ObjectiveTextList :type Array%20of%20Texts))
  (bind _wbp_objectives (Variables|Default|GetWBP_Objectives))
  ;[1 1 1] Objectives List HUD
  (if (Utilities|IsValid _wbp_objectives)
    (Default|UpdateObjectiveList _wbp_objectives ObjectiveTextList)))

(fn ConstructionScript)