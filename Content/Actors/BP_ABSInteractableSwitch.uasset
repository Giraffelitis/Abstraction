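; BP_ABSInteractableSwitch is an interactable switch that toggles its mesh between closed and open positions, optionally locked behind a key.
; When secured, Interact only proceeds if the instigator pawn's ABSActionComponent has the exact RequiredKey tag in its active gameplay tags.
; A FlipFlop alternates between playing and reversing a Timeline, whose pitch curve scales TargetOpenAngle to set SwitchMesh's relative rotation.
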(event EventInteract
  (params (InstigatorPawn :type Pawn%20Object%20Reference))
  (if (Variables|Default|GetIsSecured)
    (if (GameplayTags|HasTag (Variables|/Script/Abstraction.ABSActionComponent|GetActiveGameplayTags (Actor|GetComponentbyClass InstigatorPawn "/Script/Abstraction.ABSActionComponent")) (Variables|Default|GetRequiredKey) true)
      (Utilities|FlowControl|FlipFlop :!label _label
        (:A
          (bind _pitch (Timeline|Timeline Play)
            (:Update
              (Transformation|SetRelativeRotation (Variables|Default|GetSwitchMesh) (Math|Rotator|MakeRotator 0.0 (* _pitch (Variables|Default|GetTargetOpenAngle)) 0.0) false false))))
        (:B
          (Timeline|Timeline Reverse))))
    (else
      (goto _label))))

(fn ConstructionScript)