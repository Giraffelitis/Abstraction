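; BP_ABSInteractableButton is an interactable button that toggles between pressed and released on each Interact.
; When secured, it only responds if the instigator's ABSActionComponent holds the RequiredKey gameplay tag.
; A FlipFlop plays or reverses a timeline that slides the button mesh along local X and swaps its material between green for pressed and red for released.
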(event EventInteract
  (params (InstigatorPawn :type Pawn%20Object%20Reference))
  (bind _buttonmesh (Variables|Default|GetButtonMesh))
  (bind _buttonmesh_2 (Variables|Default|GetButtonMesh))
  (bind _relativelocation (Variables|/Script/Engine.SceneComponent|GetRelativeLocation _buttonmesh_2))
  (if (Variables|Default|GetIsSecured)
    (if (GameplayTags|HasTag (Variables|/Script/Abstraction.ABSActionComponent|GetActiveGameplayTags (Actor|GetComponentbyClass InstigatorPawn "/Script/Abstraction.ABSActionComponent")) (Variables|Default|GetRequiredKey) true)
      (Utilities|FlowControl|FlipFlop :!label _label
        (:A
          (Variables|Default|SetbIsPressed true)
          (bind _depress (Timeline|Timeline Play)
            (:Update
              (Transformation|SetRelativeLocation (Variables|Default|GetButtonMesh) (Math|Vector|MakeVector (+ (* _depress (Variables|Default|GetDepressDepthS)) 12.0) (.y _relativelocation) (.z _relativelocation)) false false)
              (if (Variables|Default|GetbIsPressed)
                (Rendering|Material|SetMaterial _buttonmesh 0 "/Game/Materials/M_Green_Shiny.M_Green_Shiny")
                (else
                  (Rendering|Material|SetMaterial _buttonmesh 0 "/Game/Materials/M_Red_Shiny.M_Red_Shiny"))))))
        (:B
          (Variables|Default|SetbIsPressed false)
          (Timeline|Timeline Reverse))))
    (else
      (goto _label))))

(fn ConstructionScript)