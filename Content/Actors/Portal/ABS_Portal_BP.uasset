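; Portal actor Blueprint that displays a render texture on its portal mesh.
; On BeginPlay it sets its target, then creates a dynamic instance of the ABSPortal_M material on the mesh with an empty portal texture.
; SetRTT feeds a valid render texture into the material's Portal_T parameter, and ClearRTT resets that parameter to empty.
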(event EventBeginPlay
  (Class|ABSPortal|SetTarget (Class|ABSPortal|GetTarget))
  (bind _returnvalue (Rendering|Material|CreateDynamicMaterialInstance (Variables|Default|GetPortalMesh) 0 "/Game/Actors/Portal/ABSPortal_M.ABSPortal_M" "None" :!class /Script/Engine.PrimitiveComponent))
  (bind _output_get (Variables|Default|SetMaterialInstance _returnvalue))
  (Rendering|Material|SetTextureParameterValue _output_get "Portal_T" 0))

(event EventSetRTT
  (params (RenderTexture :type Texture%20Object%20Reference))
  (Utilities|IsValid RenderTexture
    (:Is%20Valid
      (Rendering|Material|SetTextureParameterValue (Variables|Default|GetMaterialInstance) "Portal_T" RenderTexture))))

(event EventClearRTT
  (Rendering|Material|SetTextureParameterValue (Variables|Default|GetMaterialInstance) "Portal_T" 0))

(fn ConstructionScript)