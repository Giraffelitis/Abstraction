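; Interactable door actor that swings open and closed on alternate Interact calls.
; A FlipFlop plays or reverses the DoorSwing timeline, whose Yaw track scales TargetOpenAngle to rotate DoorMesh.
; A RequiredKey gameplay tag check on the instigator's ABSActionComponent exists, but a constant false branch bypasses it, so the door works without a key.
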(event EventInteract
  (params (InstigatorPawn :type Pawn%20Object%20Reference))
  (if false
    (if (GameplayTags|HasTag (Variables|/Script/Abstraction.ABSActionComponent|GetActiveGameplayTags (Actor|GetComponentbyClass InstigatorPawn "/Script/Abstraction.ABSActionComponent")) (Variables|Default|GetRequiredKey) true)
      (Utilities|FlowControl|FlipFlop :!label _label
        (:A
          (bind _yaw (Timeline|DoorSwing Play)
            (:Update
              (Transformation|SetRelativeRotation (Variables|Default|GetDoorMesh) (Math|Rotator|MakeRotator 0.0 0.0 (* _yaw (Variables|Default|GetTargetOpenAngle))) false false))))
        (:B
          (Timeline|DoorSwing Reverse))))
    (else
      (goto _label))))

(fn ConstructionScript)